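; Behavior tree task that has a child AI eat the candy held in its blackboard Target, which is an EnemyBase actor.
; On execute, it applies one point of damage to the ChildController itself and damage equal to the target's current health to the target.
; It then clears the Target key and finishes with success, or fails when the target is not an EnemyBase.
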(event `self.ReceiveExecute`
  (params (OwnerActor :type "Actor Object Reference"))
  (bind _aschild_controller (cast `/Game/Blueprints/AI/ChildController` OwnerActor))
  (bind _asenemy_base (cast `/Game/Blueprints/Enemies/EnemyBase` (`BTFunctionLibrary.GetBlackboardValueAsActor` (`self.Target`)))
    (:`then`
      (`GameplayStatics.ApplyDamage` _aschild_controller 1.0)
      (`GameplayStatics.ApplyDamage` _asenemy_base (`/Game/Blueprints/Player/HealthComponent.Health` (`/Game/Blueprints/Player/Character_Base.HealthComponent` _asenemy_base)))
      (`BTFunctionLibrary.SetBlackboardValueAsObject` (`self.Target`)) ; Clear our blackboard value
      (`self.FinishExecute` true))
    (:`CastFailed`
      (`self.FinishExecute` false))))
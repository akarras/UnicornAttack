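; Behavior Tree task that picks a new random wander location for an AI around its home position.
; It scales a random unit vector by WanderRadius, zeroes the Z offset and adds the home location read from the Blackboard.
; It writes the result to the target location key and finishes successfully at once, with no navmesh or reachability check.
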(event `self.ReceiveExecuteAI`
  (params (OwnerController :type "AIController Object Reference") (ControlledPawn :type "Pawn Object Reference"))
  ;[1 1 1] Gets a random location
  (`BTFunctionLibrary.SetBlackboardValueAsVector` (`self.TargetLocationKey`) (+ (`KismetMathLibrary.MakeVector` (.x (* (`KismetMathLibrary.RandomUnitVector`) (`self.WanderRadius`))) (.y (* (`KismetMathLibrary.RandomUnitVector`) (`self.WanderRadius`)))) (`BTFunctionLibrary.GetBlackboardValueAsVector` (`self.HomeLocationKey`))))
  (`self.FinishExecute` true))
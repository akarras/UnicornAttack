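; Behavior tree service that searches for the nearest actor tagged "Child" and writes it to a target blackboard key.
; On search start and each tick, it compares tagged actors' distances to the SelfActor, reading each closer child's AI blackboard to skip those with a follow target.
; The cached closest actor persists between runs, while the best distance resets after each loop.
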(event `self.ReceiveSearchStartAI`
  (params (OwnerController :type "AIController Object Reference") (ControlledPawn :type "Pawn Object Reference"))
  (bind _outactors (`GameplayStatics.GetAllActorsWithTag` "Child" :!label _label))
  (for _array_element _outactors
    (`/Engine/EditorBlueprintResources/StandardMacros.IsValid` (`self.ClosestActor`)
      (:`Is Valid`
        (bind _returnvalue (`KismetMathLibrary.VSize` (- (`Actor.K2_GetActorLocation` (`BTFunctionLibrary.GetBlackboardValueAsActor` (`self.SelfActor`))) (`Actor.K2_GetActorLocation` _array_element))))
        (if (< _returnvalue (`self.CurrentBestLength`))
          (bind _aschild (cast `/Game/Blueprints/Player/Child` _array_element))
          (bind _asaicontroller (cast `AIController` (`Pawn.GetController` _aschild)))
          (`/Engine/EditorBlueprintResources/StandardMacros.IsValid` (`BlackboardComponent.GetValueAsObject` (`AIBlueprintHelperLibrary.GetBlackboard` _asaicontroller) (`self.FollowTarget`))
            (:`Is Valid`
              (`BTFunctionLibrary.SetBlackboardValueAsObject` (`self.TargetKey`)))
            (:`Is Not Valid`
              (set `self.CurrentBestLength` _returnvalue)
              (set `self.ClosestActor` _array_element)))))
      (:`Is Not Valid`
        (set `self.ClosestActor` _array_element))))
  (set `self.CurrentBestLength` 90000.0)
  (`BTFunctionLibrary.SetBlackboardValueAsObject` (`self.TargetKey`) (`self.ClosestActor`)))

(event `self.ReceiveTickAI`
  (params (OwnerController :type "AIController Object Reference") (ControlledPawn :type "Pawn Object Reference") (DeltaSeconds :type "Float (single-precision)"))
  (goto _label))
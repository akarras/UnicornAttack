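; LaserProjectile is a projectile actor that damages enemy characters it touches.
; Capsule overlaps ignore the instigator, then apply fixed damage to any Character_Base tagged Enemy, crediting the instigator as damage causer.
; The projectile destroys itself after such a hit or when its ProjectileMovement component stops, and passes through other overlapping actors without effect.
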(event `self.Capsule.OnComponentBeginOverlap`
  (params (OverlappedComponent :type "PrimitiveComponent Object Reference") (OtherActor :type "Actor Object Reference") (OtherComp :type "PrimitiveComponent Object Reference") (OtherBodyIndex :type Integer) (bFromSweep :type Boolean) (SweepResult :type "HitResult Structure (by ref)"))
  (bind _returnvalue (`self.GetInstigator`))
  (if (!= OtherActor _returnvalue)
    (bind _ascharacter_base (cast `/Game/Blueprints/Player/Character_Base` OtherActor))
    (if (`KismetArrayLibrary.Array_Contains` (`Actor.Tags` _ascharacter_base) "Enemy")
      (`GameplayStatics.ApplyDamage` _ascharacter_base 100.0 null _returnvalue)
      (`self.K2_DestroyActor`))))

(event `self.ProjectileMovement_0.OnProjectileStop`
  (params (ImpactResult :type "HitResult Structure (by ref)"))
  (`self.K2_DestroyActor`))

(fn `UserConstructionScript`)
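; RainbowMissile_Projectile is a weapon projectile that explodes on characters tagged Enemy.
; When its capsule overlaps a Character_Base other than the instigator that carries that tag, it applies radial damage with falloff from the sphere's location.
; Minimum damage scales from the Damage variable.
; It then spawns the RainbowSplosion emitter and destroys itself, while stopping of the projectile movement destroys it without damage or effect.
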(event `self.Capsule.OnComponentBeginOverlap`
  (params (OverlappedComponent :type "PrimitiveComponent Object Reference") (OtherActor :type "Actor Object Reference") (OtherComp :type "PrimitiveComponent Object Reference") (OtherBodyIndex :type Integer) (bFromSweep :type Boolean) (SweepResult :type "HitResult Structure (by ref)"))
  (bind _damage (`self.Damage`))
  (bind _returnvalue (`SceneComponent.K2_GetComponentLocation` (`self.Sphere`)))
  (if (!= OtherActor (`self.GetInstigator`))
    (bind _ascharacter_base (cast `/Game/Blueprints/Player/Character_Base` OtherActor))
    (if (`KismetArrayLibrary.Array_Contains` (`Actor.Tags` _ascharacter_base) "Enemy")
      (`GameplayStatics.ApplyRadialDamageWithFalloff` _damage (* _damage 0.75) _returnvalue 15.0 60.0 2.0)
      (`GameplayStatics.SpawnEmitterAtLocation` "/Game/Particles/RainbowSplosion.RainbowSplosion" _returnvalue)
      (`self.K2_DestroyActor`))))

(event `self.ProjectileMovement_0.OnProjectileStop`
  (params (ImpactResult :type "HitResult Structure (by ref)"))
  (`self.K2_DestroyActor`))

(fn `UserConstructionScript`)
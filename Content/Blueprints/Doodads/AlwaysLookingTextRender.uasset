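; A floating world text doodad that turns to face the local view and fades out over its lifespan.
; Each Tick it yaws toward the camera of player 0's Character_Base pawn, staying upright.
; It also drives a dynamic font material's Opacity from remaining over initial lifespan, reapplying that material to the TextRender every frame.
; InputText sets the displayed string at construction and again through its OnRep for replication.
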(event `self.ReceiveBeginPlay`
  (bind _returnvalue (`KismetMaterialLibrary.CreateDynamicMaterialInstance` "/Game/Materials/FontMatWithOpacity.FontMatWithOpacity"))
  (set `self.FontMat` _returnvalue))

(event `self.ReceiveTick`
  (params (DeltaSeconds :type "Float (single-precision)"))
  (bind _fontmat (`self.FontMat`))
  (bind _ascharacter_base (cast `/Game/Blueprints/Player/Character_Base` (`GameplayStatics.GetPlayerPawn` 0)))
  (`SceneComponent.K2_SetWorldRotation` (`self.DefaultSceneRoot`) (`KismetMathLibrary.MakeRotator` 0.0 0.0 (.yaw (`KismetMathLibrary.FindLookAtRotation` (`self.K2_GetActorLocation`) (`SceneComponent.K2_GetComponentLocation` (`/Game/Blueprints/Player/Character_Base.Camera` _ascharacter_base))))) false false)
  (`MaterialInstanceDynamic.SetScalarParameterValue` _fontmat "Opacity" (/ (`self.GetLifeSpan`) (`self.InitialLifeSpan`)))
  (`TextRenderComponent.SetTextMaterial` (`self.TextRender`) _fontmat))

(fn `OnRep_InputText`
  (`TextRenderComponent.K2_SetText` (`self.TextRender`) (`self.InputText`)))

(fn `UserConstructionScript`
  (`TextRenderComponent.K2_SetText` (`self.TextRender`) (`self.InputText`)))
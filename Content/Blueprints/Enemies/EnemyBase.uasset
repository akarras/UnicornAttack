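; EnemyBase is the base enemy actor with a floating health bar that reports its removal to the game mode.
; Each tick it copies HealthComponent health and max health into the Healthbar widget and turns the widget, yaw only, toward the player's Character_Base camera.
; On Destroyed it decrements EnemiesAlive on UnicornGamemode and calls CheckRoundState to update the round.
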(event `self.ReceiveBeginPlay`)

(event `self.ReceiveTick`
  (params (DeltaSeconds :type "Float (single-precision)"))
  (bind _healthcomponent (`self.HealthComponent`))
  (`parent.ReceiveTick` DeltaSeconds)
  (bind _ashealthbar (cast `/Game/Blueprints/UI/Healthbar` (`WidgetComponent.GetUserWidgetObject` (`self.HealthWidget`))))
  (set `/Game/Blueprints/UI/Healthbar.Health` (`/Game/Blueprints/Player/HealthComponent.Health` _healthcomponent) _ashealthbar)
  (set `/Game/Blueprints/UI/Healthbar.MaxHealth` (`/Game/Blueprints/Player/HealthComponent.MaxHealth` _healthcomponent) _ashealthbar)
  (bind _ascharacter_base (cast `/Game/Blueprints/Player/Character_Base` (`GameplayStatics.GetPlayerPawn` 0)))
  (`SceneComponent.K2_SetWorldRotation` (`self.HealthWidget`) (`KismetMathLibrary.MakeRotator` 0.0 0.0 (.yaw (`KismetMathLibrary.FindLookAtRotation` (`self.K2_GetActorLocation`) (`SceneComponent.K2_GetComponentLocation` (`/Game/Blueprints/Player/Character_Base.Camera` _ascharacter_base))))) false false))

(event `self.ReceiveDestroyed`
  (bind _asunicorn_gamemode (cast `/Game/Blueprints/Game/UnicornGamemode` (`GameplayStatics.GetGameMode`)))
  (`/Engine/EditorBlueprintResources/StandardMacros.DecrementInt` (`/Game/Blueprints/Game/UnicornGamemode.EnemiesAlive` _asunicorn_gamemode)
    (:`  `
      (`/Game/Blueprints/Game/UnicornGamemode.CheckRoundState` _asunicorn_gamemode))))

(fn `UserConstructionScript`
  (`parent.UserConstructionScript`))
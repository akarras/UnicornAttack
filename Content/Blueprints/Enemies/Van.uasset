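; Van is an enemy spawn point that releases waves of enemies at the start of each round.
; On BeginPlay it binds to the UnicornGamemode new-round event.
; Each round it adds that wave's enemy count to the gamemode's round total and sets the alive count to it.
; It then spawns every class in the round's Waves entry at its own transform, adjusting for collisions but always spawning.
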(event `self.ReceiveBeginPlay`
  ;[1 1 1] Bind our New Round event to the GameMode
  (bind _asunicorn_gamemode (cast `/Game/Blueprints/Game/UnicornGamemode` (`GameplayStatics.GetGameMode`)))
  (add `/Game/Blueprints/Game/UnicornGamemode.NewRound` _asunicorn_gamemode (delegate `NewRound`)))

(event `NewRound`
  (params (RoundNumber :type Integer))
  (bind _enemies (break `/Game/Blueprints/Enemies/Waves` (`KismetArrayLibrary.Array_Get` (`self.Waves`) (- RoundNumber 1))))
  (bind _asunicorn_gamemode (cast `/Game/Blueprints/Game/UnicornGamemode` (`GameplayStatics.GetGameMode`)))
  (bind _output_get (set `/Game/Blueprints/Game/UnicornGamemode.EnemiesThisRound` (+ (`/Game/Blueprints/Game/UnicornGamemode.EnemiesThisRound` _asunicorn_gamemode) (`KismetArrayLibrary.Array_Length` _enemies)) _asunicorn_gamemode))
  (set `/Game/Blueprints/Game/UnicornGamemode.EnemiesAlive` _output_get _asunicorn_gamemode)
  (for _array_element _enemies
    (`|SpawnActorFromClass` _array_element (`self.GetTransform`) "AdjustIfPossibleButAlwaysSpawn" "OverrideRootScale")
    (`KismetSystemLibrary.PrintString` "Spawned")))

(fn `UserConstructionScript`)
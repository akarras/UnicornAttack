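; Game mode that runs the wave loop, alternating timed Shop and Round phases and returning to the main menu when no children remain alive.
; A looping one-second timer advances expired phases, while CheckRoundState ends rounds early once enemies are gone.
; The NewRound dispatcher sets each phase's duration and copies round state and timing to UnicornGameState.
; It also configures UnicornController UI on login and controller swap.
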(event `self.K2_OnSwapPlayerControllers`
  (params (OldPC :type "PlayerController Object Reference") (NewPC :type "PlayerController Object Reference"))
  (bind _asunicorn_controller (cast `/Game/Blueprints/Player/UnicornController` NewPC))
  (`/Game/Blueprints/Player/UnicornController.ConfigureUI` _asunicorn_controller))

(event `self.K2_PostLogin`
  (params (NewPlayer :type "PlayerController Object Reference"))
  (bind _asunicorn_controller (cast `/Game/Blueprints/Player/UnicornController` NewPlayer))
  (`/Game/Blueprints/Player/UnicornController.ConfigureUI` _asunicorn_controller))

(event `self.ReceiveBeginPlay`
  ;[1 1 1] Round Over
  (`KismetSystemLibrary.Delay` 2.0)
  (`self.RoundOver`)
  (add `self.NewRound` (delegate `NewRound_Event`))
  (`KismetSystemLibrary.K2_SetTimer` null "RoundTimeTick" 1.0 true))

(event `NewRound_Event` :!signature `self.NewRound`
  (params (RoundNumber :type Integer) (NewRoundState :type "/Game/Blueprints/Game/RoundState Enum"))
  (bind _output_get (set `self.RoundTime` (select `/Game/Blueprints/Game/RoundState` NewRoundState :`NewEnumerator0` 15.0 :`NewEnumerator1` 90.0 :`NewEnumerator2` 30.0 :`NewEnumerator3` 15.0 :!type "Float (single-precision)")))
  (bind _output_get_2 (set `self.RoundGameTime` (`KismetSystemLibrary.GetGameTimeInSeconds`)))
  (bind _asunicorn_game_state (cast `/Game/Blueprints/Game/UnicornGameState` (`GameplayStatics.GetGameState`)))
  (set `/Game/Blueprints/Game/UnicornGameState.RoundTime` _output_get _asunicorn_game_state)
  (set `/Game/Blueprints/Game/UnicornGameState.RoundGameTime` _output_get_2 _asunicorn_game_state)
  (set `/Game/Blueprints/Game/UnicornGameState.CurrentRound` (`self.CurrentRound`) _asunicorn_game_state)
  (set `/Game/Blueprints/Game/UnicornGameState.RoundState` (`self.RoundState`) _asunicorn_game_state))

(event `RoundOver`
  ;[1 1 1] Update round
  (set `self.RoundState` "NewEnumerator2")
  (set `self.EnemiesThisRound` 0)
  (`self.NewRound` (`self.CurrentRound`) (`self.RoundState`)))

(event `CheckRoundState`
  ;[1 1 1] Check if the round should end
  (switch `/Game/Blueprints/Game/RoundState` (`self.RoundState`)
    (:`NewEnumerator1`
      (if (== (`self.EnemiesAlive`) 0)
        (`self.RoundOver`)))))

(event `CheckGameLose`
  ;[1 1 1] Game Lose
  (if (<= (`self.ChildrenAlive`) 0)
    (set `self.RoundState` "NewEnumerator3")
    (`GameplayStatics.OpenLevel` "MainMenu")))

(fn `GetTimeLeftInRound`
  (returns (TimeLeft :type "Float (double-precision)"))
  (return (- (`self.RoundTime`) (- (`KismetSystemLibrary.GetGameTimeInSeconds`) (`self.RoundGameTime`)))))

(fn `RoundTimeTick`
  (bind _timeleft (`self.GetTimeLeftInRound`))
  (if (< _timeleft 0.0)
    (bind _output_get (set `self.RoundState` (select `/Game/Blueprints/Game/RoundState` (`self.RoundState`) :`NewEnumerator0` "NewEnumerator2" :`NewEnumerator1` "NewEnumerator2" :`NewEnumerator2` "NewEnumerator1" :`NewEnumerator3` "NewEnumerator3" :!type "/Game/Blueprints/Game/RoundState Enum")))
    (switch `/Game/Blueprints/Game/RoundState` _output_get
      (:`NewEnumerator0`
        _)
      (:`NewEnumerator1`
        (set `self.CurrentRound` (+ (`self.CurrentRound`) 1)))
      (:`NewEnumerator2`
        _)
      (:`NewEnumerator3`
        _))
    (`self.NewRound` (`self.CurrentRound`) _output_get)))

(fn `UserConstructionScript`)
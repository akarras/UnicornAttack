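; CandyEssence is a money pickup that homes in on a unicorn and adds its value to that unicorn's Money.
; On BeginPlay it scans all Unicorn_Base actors and locks onto the nearest one.
; Each tick it moves a fixed step toward that target, without sweeping or delta-time scaling.
; Any Unicorn_Base overlapping its sphere receives the money, then the pickup destroys itself.
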(event `self.ReceiveBeginPlay`
  (bind _closestplayer (`self.GetClosestUser`))
  (set `self.Unicorn` _closestplayer))

(event `self.ReceiveTick`
  (params (DeltaSeconds :type "Float (single-precision)"))
  ;[1 1 1] Move to the other object
  (`self.K2_AddActorWorldOffset` (* (`KismetMathLibrary.GetDirectionVector` (`self.K2_GetActorLocation`) (`self.K2_GetActorLocation` (`self.Unicorn`))) 40.0)))

(event `self.Sphere.OnComponentBeginOverlap`
  (params (OverlappedComponent :type "PrimitiveComponent Object Reference") (OtherActor :type "Actor Object Reference") (OtherComp :type "PrimitiveComponent Object Reference") (OtherBodyIndex :type Integer) (bFromSweep :type Boolean) (SweepResult :type "HitResult Structure (by ref)"))
  ;[1 1 1] Pick up the money
  (bind _asunicorn_base (cast `/Game/Blueprints/Player/Unicorn_Base` OtherActor))
  (set `/Game/Blueprints/Player/Character_Base.Money` (+ (`self.Money`) (`/Game/Blueprints/Player/Character_Base.Money` _asunicorn_base)) _asunicorn_base)
  (`self.K2_DestroyActor`))

(fn `GetClosestUser`
  (returns (ClosestPlayer :type "/Game/Blueprints/Player/Unicorn_Base Object Reference"))
  (locals (ClosestLength :type "Float (double-precision)") (CurrentClosest :type "/Game/Blueprints/Player/Unicorn_Base Object Reference"))
  (bind _outactors (`GameplayStatics.GetAllActorsOfClass` "/Game/Blueprints/Player/Unicorn_Base.Unicorn_Base_C"))
  (bind _item (`KismetArrayLibrary.Array_Get` _outactors))
  (bind _length (`self.GetDistance` _item))
  (set `local.ClosestLength` _length)
  (set `local.CurrentClosest` _item)
  (for _array_element _outactors
    (bind _length_2 (`self.GetDistance` _array_element))
    (if (> (`local.ClosestLength`) _length_2)
      (set `local.ClosestLength` _length_2)
      (set `local.CurrentClosest` _array_element)))
  (return (`local.CurrentClosest`)))

(fn `GetDistance`
  (params (OtherActor :type "Actor Object Reference"))
  (returns (Length :type "Float (double-precision)"))
  (return (`KismetMathLibrary.VSize` (- (`self.K2_GetActorLocation`) (`self.K2_GetActorLocation` OtherActor)))))

(fn `UserConstructionScript`)
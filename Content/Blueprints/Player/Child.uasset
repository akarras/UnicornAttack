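; Child actor whose survival counts toward the game's lose condition.
; On BeginPlay it increments ChildrenAlive on the UnicornGamemode.
; When destroyed it decrements that count and calls CheckGameLose on the game mode to see if losing this child ends the game.
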(event `self.ReceiveBeginPlay`
  (bind _asunicorn_gamemode (cast `/Game/Blueprints/Game/UnicornGamemode` (`GameplayStatics.GetGameMode`)))
  (set `/Game/Blueprints/Game/UnicornGamemode.ChildrenAlive` (+ (`/Game/Blueprints/Game/UnicornGamemode.ChildrenAlive` _asunicorn_gamemode) 1) _asunicorn_gamemode))

(event `self.ReceiveDestroyed`
  (bind _asunicorn_gamemode (cast `/Game/Blueprints/Game/UnicornGamemode` (`GameplayStatics.GetGameMode`)))
  (set `/Game/Blueprints/Game/UnicornGamemode.ChildrenAlive` (- (`/Game/Blueprints/Game/UnicornGamemode.ChildrenAlive` _asunicorn_gamemode) 1) _asunicorn_gamemode)
  (bind _asunicorn_gamemode_2 (cast `/Game/Blueprints/Game/UnicornGamemode` (`GameplayStatics.GetGameMode`)))
  (`/Game/Blueprints/Game/UnicornGamemode.CheckGameLose` _asunicorn_gamemode_2) ; Check if losing this child should lose the player the game
)

(fn `UserConstructionScript`
  (`parent.UserConstructionScript`))